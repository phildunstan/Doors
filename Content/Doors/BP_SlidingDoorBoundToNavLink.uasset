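; Sliding door actor that opens for AI reaching its smart nav link and also exposes open, close and toggle events.
; A timeline slides the door mesh along the actor's local X axis from its starting position.
; A nav modifier volume switches area class, treating the door as closed while moving and open once fully open.
; The agent stops at a closed door and resumes path following when the door-open event fires.
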(event `self.ReceiveBeginPlay`
  (`|ExecutionSequence`
    (:`then_0`
      (set `self.ClosedDoorPosition` (`self.K2_GetActorLocation`)))
    (:`then_1`
      ; Update the door position if the door starts open
      (if (`self.bIsOpen`)
        (`TimelineComponent.SetNewTime` (`self.Door Animation Timeline`) 100.0)))
    (:`then_2`
      ; Update the navmesh override volume
      (`/Engine/EditorBlueprintResources/StandardMacros.IsValid` (`self.NavModifierVolume`)
        (:`Is Valid`
          (if (`self.bIsOpen`)
            (`NavModifierVolume.SetAreaClass` (`self.NavModifierVolume`) (`self.NavAreaClassOpenDoor`))
            (else
              (`NavModifierVolume.SetAreaClass` (`self.NavModifierVolume`) (`self.NavAreaClassClosedDoor`)))))))
    (:`then_3`
      (add `NavLinkProxy.OnSmartLinkReached` (`self.NavLink`) (delegate `Handle On Smart Link Reached`)))))

(event `Handle On Smart Link Reached`
  (params (MovingActor :type "Actor Object Reference") (DestinationPoint :type "Vector Structure (by ref)"))
  (if (not (`self.bIsOpen`))
    (add `self.On Door Open` (delegate `Handle On Door Open`))
    (`Controller.StopMovement` (`AIBlueprintHelperLibrary.GetAIController` MovingActor))
    (`DoorInterface.OpenDoor`)
    (else
      (`NavLinkProxy.ResumePathFollowing` (`self.NavLink`) MovingActor))))

(event `Handle On Door Open`
  (remove `self.On Door Open` (delegate `Handle On Door Open`))
  (`NavLinkProxy.ResumePathFollowing` (`self.NavLink`) (stale `Handle On Smart Link Reached` MovingActor)))

(event `DoorInterface.OpenDoor`
  (if (`TimelineComponent.IsPlaying` (`self.Door Animation Timeline`))
    _
    (elif (not (`self.bIsOpen`))
      (`TimelineComponent.Play` (`self.Door Animation Timeline`)))))

(event `DoorInterface.CloseDoor`
  (if (`TimelineComponent.IsPlaying` (`self.Door Animation Timeline`))
    _
    (elif (`self.bIsOpen`)
      (set `self.bIsOpen` false)
      (`TimelineComponent.Reverse` (`self.Door Animation Timeline`)))))

(event `DoorInterface.ToggleDoorOpenOrClosed`
  (if (`TimelineComponent.IsPlaying` (`self.Door Animation Timeline`))
    _
    (elif (`self.bIsOpen`)
      (`DoorInterface.CloseDoor`)
      (else
        (`DoorInterface.OpenDoor`)))))

(fn `IsDoorOpen`
  (returns (ReturnValue :type Boolean))
  (return (`self.bIsOpen`)))

(fn `UserConstructionScript`)