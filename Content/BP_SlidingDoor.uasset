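; Sliding door actor that automatically toggles open and closed on a repeating two-second delay after BeginPlay.
; BeginPlay stores the closed position and jumps the Timeline to its end when starting open.
; Open and Close play or reverse the Timeline, ignoring calls while it is playing.
; Timeline updates offset the door mesh from the closed position along the actor's local X axis.
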(event `self.ReceiveBeginPlay`
  (`|ExecutionSequence`
    (:`then_0`
      (set `self.ClosedDoorPosition` (`self.K2_GetActorLocation`)))
    (:`then_1`
      (if (`self.bIsOpen`)
        (`TimelineComponent.SetNewTime` (`self.Timeline`) 100.0)))
    (:`then_2`
      (`KismetSystemLibrary.Delay` 2.0)
      (`self.ToggleIndefinitely`))))

(event `ToggleIndefinitely`
  (`self.ToggleOpenOrClosed`)
  (`KismetSystemLibrary.Delay` 2.0)
  (`self.ToggleIndefinitely`))

(fn `Close`
  (if (`TimelineComponent.IsPlaying` (`self.Timeline`))
    _
    (elif (`self.bIsOpen`)
      (`TimelineComponent.Reverse` (`self.Timeline`))
      (set `self.bIsOpen` false))))

(fn `IsOpen`
  (returns (bIsOpen :type Boolean))
  (return (`self.bIsOpen`)))

(fn `Open`
  (if (`TimelineComponent.IsPlaying` (`self.Timeline`))
    _
    (elif (not (`self.bIsOpen`))
      (`TimelineComponent.Play` (`self.Timeline`))
      (set `self.bIsOpen` true))))

(fn `ToggleOpenOrClosed`
  (if (`TimelineComponent.IsPlaying` (`self.Timeline`))
    _
    (elif (`self.bIsOpen`)
      (`self.Close`)
      (else
        (`self.Open`)))))

(fn `UserConstructionScript`)