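; Sliding door actor that opens, closes or toggles on request and can start open, updating navigation to match its state.
; A timeline slides the door mesh along the actor's local X from its closed position, ignoring new requests while moving.
; An optional nav modifier volume switches area class, using the closed class while moving or closed and the open class once fully open.
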(event `self.ReceiveBeginPlay`
  (`|ExecutionSequence`
    (:`then_0`
      (set `self.ClosedDoorPosition` (`self.K2_GetActorLocation`)))
    (:`then_1`
      ; Update the door position if the door starts open
      (if (`self.bIsOpen`)
        (`TimelineComponent.SetNewTime` (`self.Door Animation Timeline`) 100.0)))
    (:`then_2`
      ; Update the navmesh override volume
      (`/Engine/EditorBlueprintResources/StandardMacros.IsValid` (`self.NavModifierVolume`)
        (:`Is Valid`
          (if (`self.bIsOpen`)
            (`NavModifierVolume.SetAreaClass` (`self.NavModifierVolume`) (`self.NavAreaClassOpenDoor`))
            (else
              (`NavModifierVolume.SetAreaClass` (`self.NavModifierVolume`) (`self.NavAreaClassClosedDoor`)))))))))

(event `/Game/Doors/BI_DoorInterface.Open`
  (if (`TimelineComponent.IsPlaying` (`self.Door Animation Timeline`))
    _
    (elif (not (`self.bIsOpen`))
      (`TimelineComponent.Play` (`self.Door Animation Timeline`))
      (set `self.bIsOpen` true))))

(event `/Game/Doors/BI_DoorInterface.Close`
  (if (`TimelineComponent.IsPlaying` (`self.Door Animation Timeline`))
    _
    (elif (`self.bIsOpen`)
      (`TimelineComponent.Reverse` (`self.Door Animation Timeline`))
      (set `self.bIsOpen` false))))

(event `/Game/Doors/BI_DoorInterface.ToggleOpenOrClosed`
  (if (`TimelineComponent.IsPlaying` (`self.Door Animation Timeline`))
    _
    (elif (`self.bIsOpen`)
      (`self.Close`)
      (else
        (`self.Open`)))))

(fn `IsOpen`
  (returns (bIsOpen :type Boolean))
  (return (`self.bIsOpen`)))

(fn `UserConstructionScript`)