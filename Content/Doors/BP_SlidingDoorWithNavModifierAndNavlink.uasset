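; Sliding door actor that updates navigation as it opens and closes and can open itself for AI agents.
; A timeline slides the door mesh along the actor's local X axis from its closed position.
; An optional nav modifier volume takes the closed-door area class until fully open, then the open-door class.
; Agents reaching the smart nav link at a closed door stop, trigger opening, and resume pathing after a short delay.
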(event `self.ReceiveBeginPlay`
  (`|ExecutionSequence`
    (:`then_0`
      (set `self.ClosedDoorPosition` (`self.K2_GetActorLocation`)))
    (:`then_1`
      ; Update the door position if the door starts open
      (if (`self.bIsOpen`)
        (`TimelineComponent.SetNewTime` (`self.Door Animation Timeline`) 100.0)))
    (:`then_2`
      ; Update the navmesh override volume
      (`/Engine/EditorBlueprintResources/StandardMacros.IsValid` (`self.NavModifierVolume`)
        (:`Is Valid`
          (if (`self.bIsOpen`)
            (`NavModifierVolume.SetAreaClass` (`self.NavModifierVolume`) (`self.NavAreaClassOpenDoor`))
            (else
              (`NavModifierVolume.SetAreaClass` (`self.NavModifierVolume`) (`self.NavAreaClassClosedDoor`)))))))
    (:`then_3`
      (add `NavLinkProxy.OnSmartLinkReached` (`self.NavLink`) (delegate `CustomEvent`)))))

(event `CustomEvent`
  (params (MovingActor :type "Actor Object Reference") (DestinationPoint :type "Vector Structure (by ref)"))
  (if (not (`self.bIsOpen`))
    (`Controller.StopMovement` (`AIBlueprintHelperLibrary.GetAIController` MovingActor))
    (`self.Open`)
    (`KismetSystemLibrary.Delay` 1.0)
    (`NavLinkProxy.ResumePathFollowing` (`self.NavLink`) MovingActor)
    (else
      (`NavLinkProxy.ResumePathFollowing` (`self.NavLink`) MovingActor))))

(event `/Game/Doors/BI_DoorInterface.Open`
  (if (`TimelineComponent.IsPlaying` (`self.Door Animation Timeline`))
    _
    (elif (not (`self.bIsOpen`))
      (`TimelineComponent.Play` (`self.Door Animation Timeline`)))))

(event `/Game/Doors/BI_DoorInterface.Close`
  (if (`TimelineComponent.IsPlaying` (`self.Door Animation Timeline`))
    _
    (elif (`self.bIsOpen`)
      (set `self.bIsOpen` false)
      (`TimelineComponent.Reverse` (`self.Door Animation Timeline`)))))

(event `/Game/Doors/BI_DoorInterface.ToggleOpenOrClosed`
  (if (`TimelineComponent.IsPlaying` (`self.Door Animation Timeline`))
    _
    (elif (`self.bIsOpen`)
      (`self.Close`)
      (else
        (`self.Open`)))))

(fn `IsOpen`
  (returns (bIsOpen :type Boolean))
  (return (`self.bIsOpen`)))

(fn `UserConstructionScript`)